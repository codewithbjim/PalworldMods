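; Gamepad input Blueprint for Perfect Placement that turns left-stick click (L3) taps and chords into physical-input events queued on a key guide widget.
; L3 plus D-Pad Up or Down fires one chord per hold; releasing L3 without a chord queues the tap action instead.
; Initialize supplies the widget and player controller; ActivateInput and DeactivateInput reset chord state and toggle input on that controller.
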(event Input|GamepadEvents|GamepadLeftThumbstick
  (params (Key :type Key%20Structure :default "None"))
  (bind _keyguidewidget (Variables|Default|GetKeyGuideWidget))
  (:Pressed
    (Variables|Default|SetbL3Held true)
    (Variables|Default|SetbL3CompoundChordUsed false))
  (:Released
    (if (Variables|Default|GetbL3Held)
      (Variables|Default|SetbL3Held false)
      (if (Variables|Default|GetbL3CompoundChordUsed)
        (Variables|Default|SetbL3CompoundChordUsed false)
        (else
          (Variables|Default|SetbL3CompoundChordUsed false)
          (Utilities|IsValid _keyguidewidget
            (:Is%20Valid
              (Default|QueueGamepadPhysicalInput _keyguidewidget "NewEnumerator0"))))))))

(event Input|GamepadEvents|GamepadDPadDown
  (params (Key :type Key%20Structure :default "None"))
  (bind _keyguidewidget (Variables|Default|GetKeyGuideWidget))
  (:Pressed
    (if (and (Variables|Default|GetbL3Held) (not (Variables|Default|GetbL3CompoundChordUsed)))
      (Utilities|IsValid _keyguidewidget
        (:Is%20Valid
          (Variables|Default|SetbL3CompoundChordUsed true)
          (Default|QueueGamepadPhysicalInput _keyguidewidget "NewEnumerator1"))))))

(event Input|GamepadEvents|GamepadDPadUp
  (params (Key :type Key%20Structure :default "None"))
  (bind _keyguidewidget (Variables|Default|GetKeyGuideWidget))
  (:Pressed
    (if (and (Variables|Default|GetbL3Held) (not (Variables|Default|GetbL3CompoundChordUsed)))
      (Utilities|IsValid _keyguidewidget
        (:Is%20Valid
          (Variables|Default|SetbL3CompoundChordUsed true)
          (Default|QueueGamepadPhysicalInput _keyguidewidget "NewEnumerator23"))))))

(fn ConstructionScript)

(fn Initialize
  (params (InWidget :type WBP%20Perfect%20Placement%20Key%20Guide%20Object%20Reference) (InPlayerController :type Player%20Controller%20Object%20Reference))
  (Variables|Default|SetKeyGuideWidget InWidget)
  (Variables|Default|SetPlayerController InPlayerController))

(fn ActivateInput
  (Variables|Default|SetbL3Held false)
  (Variables|Default|SetbL3CompoundChordUsed false)
  (Input|EnableInput (Variables|Default|GetPlayerController)))

(fn DeactivateInput
  (Variables|Default|SetbL3Held false)
  (Variables|Default|SetbL3CompoundChordUsed false)
  (Input|DisableInput (Variables|Default|GetPlayerController)))