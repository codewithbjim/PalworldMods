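; Gamepad input actor for Perfect Placement that forwards D-pad, shoulder and thumbstick presses to a key guide widget as queued physical-input enum values.
; Analog triggers past half pull act as held modifiers, giving each D-pad direction four variants: plain, left, right or both triggers.
; An owner supplies the widget and player controller via Initialize, then Activate/DeactivateInput toggles input on that controller and clears trigger state.
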(event Input|GamepadEvents|GamepadLeftTriggerAxis
  (params (AxisValue :type Float%20%28single-precision%29))
  (Variables|Default|SetbLeftTriggerHeld (>= AxisValue 0.5)))

(event Input|GamepadEvents|GamepadRightTriggerAxis
  (params (AxisValue :type Float%20%28single-precision%29))
  (Variables|Default|SetbRightTriggerHeld (>= AxisValue 0.5)))

(event Input|GamepadEvents|GamepadDPadRight
  (params (Key :type Key%20Structure :default "None"))
  (:Pressed
    (CallFunction|QueueFrozenDPad "NewEnumerator3")))

(event Input|GamepadEvents|GamepadDPadUp
  (params (Key :type Key%20Structure :default "None"))
  (:Pressed
    (CallFunction|QueueFrozenDPad "NewEnumerator0")))

(event Input|GamepadEvents|GamepadDPadDown
  (params (Key :type Key%20Structure :default "None"))
  (:Pressed
    (CallFunction|QueueFrozenDPad "NewEnumerator1")))

(event Input|GamepadEvents|GamepadDPadLeft
  (params (Key :type Key%20Structure :default "None"))
  (:Pressed
    (CallFunction|QueueFrozenDPad "NewEnumerator2")))

(event Input|GamepadEvents|GamepadLeftThumbstick
  (params (Key :type Key%20Structure :default "None"))
  (:Pressed
    (Default|QueueGamepadPhysicalInput (Variables|Default|GetKeyGuideWidget) "NewEnumerator21")))

(event Input|GamepadEvents|GamepadLeftShoulder
  (params (Key :type Key%20Structure :default "None"))
  (:Pressed
    (Default|QueueGamepadPhysicalInput (Variables|Default|GetKeyGuideWidget) "NewEnumerator18")))

(event Input|GamepadEvents|GamepadRightShoulder
  (params (Key :type Key%20Structure :default "None"))
  (:Pressed
    (Default|QueueGamepadPhysicalInput (Variables|Default|GetKeyGuideWidget) "NewEnumerator19")))

(event Input|GamepadEvents|GamepadRightThumbstick
  (params (Key :type Key%20Structure :default "None"))
  (:Pressed
    (Default|QueueGamepadPhysicalInput (Variables|Default|GetKeyGuideWidget) "NewEnumerator20")))

(fn ConstructionScript)

(fn Initialize
  (params (InWidget :type WBP%20Perfect%20Placement%20Key%20Guide%20Object%20Reference) (InPlayerController :type Player%20Controller%20Object%20Reference))
  (Variables|Default|SetKeyGuideWidget InWidget)
  (Variables|Default|SetPlayerController InPlayerController))

(fn ActivateInput
  (if (not (Variables|Default|GetbInputActive))
    (Variables|Default|SetbLeftTriggerHeld false)
    (Variables|Default|SetbRightTriggerHeld false)
    (Input|EnableInput (Variables|Default|GetPlayerController))
    (Variables|Default|SetbInputActive true)))

(fn DeactivateInput
  (Variables|Default|SetbLeftTriggerHeld false)
  (Variables|Default|SetbRightTriggerHeld false)
  (if (Variables|Default|GetbInputActive)
    (Input|DisableInput (Variables|Default|GetPlayerController))
    (Variables|Default|SetbInputActive false)))

(fn QueueFrozenDPad
  (params (Direction :type EPP_DPadDirection%20Enum :default "NewEnumerator0"))
  (bind _keyguidewidget (Variables|Default|GetKeyGuideWidget))
  (bind _keyguidewidget_2 (Variables|Default|GetKeyGuideWidget))
  (bind _keyguidewidget_3 (Variables|Default|GetKeyGuideWidget))
  (bind _keyguidewidget_4 (Variables|Default|GetKeyGuideWidget))
  (if (Variables|Default|GetbLeftTriggerHeld)
    (if (Variables|Default|GetbRightTriggerHeld)
      (switch Utilities|FlowControl|Switch|SwitchonEPP_DPadDirection Direction
        (:NewEnumerator0
          (Default|QueueGamepadPhysicalInput _keyguidewidget "NewEnumerator14"))
        (:NewEnumerator1
          (Default|QueueGamepadPhysicalInput _keyguidewidget "NewEnumerator15"))
        (:NewEnumerator2
          (Default|QueueGamepadPhysicalInput _keyguidewidget "NewEnumerator16"))
        (:NewEnumerator3
          (Default|QueueGamepadPhysicalInput _keyguidewidget "NewEnumerator17")))
      (else
        (switch Utilities|FlowControl|Switch|SwitchonEPP_DPadDirection Direction
          (:NewEnumerator0
            (Default|QueueGamepadPhysicalInput _keyguidewidget_2 "NewEnumerator6"))
          (:NewEnumerator1
            (Default|QueueGamepadPhysicalInput _keyguidewidget_2 "NewEnumerator7"))
          (:NewEnumerator2
            (Default|QueueGamepadPhysicalInput _keyguidewidget_2 "NewEnumerator8"))
          (:NewEnumerator3
            (Default|QueueGamepadPhysicalInput _keyguidewidget_2 "NewEnumerator9")))))
    (elif (Variables|Default|GetbRightTriggerHeld)
      (switch Utilities|FlowControl|Switch|SwitchonEPP_DPadDirection Direction
        (:NewEnumerator0
          (Default|QueueGamepadPhysicalInput _keyguidewidget_4 "NewEnumerator10"))
        (:NewEnumerator1
          (Default|QueueGamepadPhysicalInput _keyguidewidget_4 "NewEnumerator11"))
        (:NewEnumerator2
          (Default|QueueGamepadPhysicalInput _keyguidewidget_4 "NewEnumerator12"))
        (:NewEnumerator3
          (Default|QueueGamepadPhysicalInput _keyguidewidget_4 "NewEnumerator13")))
      (else
        (switch Utilities|FlowControl|Switch|SwitchonEPP_DPadDirection Direction
          (:NewEnumerator0
            (Default|QueueGamepadPhysicalInput _keyguidewidget_3 "NewEnumerator2"))
          (:NewEnumerator1
            (Default|QueueGamepadPhysicalInput _keyguidewidget_3 "NewEnumerator3"))
          (:NewEnumerator2
            (Default|QueueGamepadPhysicalInput _keyguidewidget_3 "NewEnumerator4"))
          (:NewEnumerator3
            (Default|QueueGamepadPhysicalInput _keyguidewidget_3 "NewEnumerator5")))))))